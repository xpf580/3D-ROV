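; Showcase variant of the East Sovremenny ship Blueprint that exposes the vessel's moving parts and weapons to generic slider, button and checkbox events.
; Sliders drive lights, propellers, rudder, sensor base and weapon aiming, with small guns and rockets sharing one elevation and rotation pair.
; Buttons fire either main gun or all four small guns together, and a checkbox toggles the damaged look.
; BeginPlay starts the three radars spinning.
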(event EventBeginPlay
  (|CallParentFunction)
  (CallFunction|SetRadarCenterSpeed 1.0)
  (CallFunction|SetRadarLeftSpeed 1.0)
  (CallFunction|SetRadarRightSpeed 1.0))

(event Collision|EventActorBeginOverlap
  (params (OtherActor :type Actor%20Object%20Reference))
  (|CallParentFunction OtherActor) ; This node is disabled and will not be called.\nDrag off pins to build functionality.
)

(event EventSetTwinSliderVariable6
  (params (bFirstSlider? :type Boolean) (NewFirstValue :type Float%20%28single-precision%29) (NewSecondValue :type Float%20%28single-precision%29))
  (CallFunction|SetSensorBaseRotation NewFirstValue)
  (CallFunction|SetRudder NewSecondValue))

(event EventSetButtonsVariable0
  (params (NewIndex :type Integer))
  (switch int NewIndex
    (:0
      (CallFunction|FireFrontMainGun))
    (:1
      (CallFunction|FirerearMainGun))))

(event EventSetButtonsVariable1
  (params (NewIndex :type Integer))
  (CallFunction|FireSmallGunFrontLeft)
  (CallFunction|FireSmallGunFrontRight)
  (CallFunction|FireSmallGunRearLeft)
  (CallFunction|FireSmallGunRearRight))

(event EventSetCheckboxVariable0
  (params (NewState :type Boolean))
  (CallFunction|SetShowDamaged NewState))

(event EventTick
  (params (DeltaSeconds :type Float%20%28single-precision%29))
  (|CallParentFunction DeltaSeconds) ; This node is disabled and will not be called.\nDrag off pins to build functionality.
)

(event EventSetTwinSliderVariable0
  (params (bFirstSlider? :type Boolean) (NewFirstValue :type Float%20%28single-precision%29) (NewSecondValue :type Float%20%28single-precision%29))
  (CallFunction|SetLeftPropellerSpeed NewFirstValue)
  (CallFunction|SetRightPropellerSpeed NewSecondValue))

(event EventSetTwinSliderVariable1
  (params (bFirstSlider? :type Boolean) (NewFirstValue :type Float%20%28single-precision%29) (NewSecondValue :type Float%20%28single-precision%29))
  (CallFunction|SetFrontGunElevation NewFirstValue)
  (CallFunction|SetFrontGunBaseRotation NewSecondValue))

(event EventSetSliderVariable0
  (params (NewValue :type Float%20%28single-precision%29))
  (CallFunction|SetLightsEmissivity NewValue))

(event EventSetTwinSliderVariable2
  (params (bFirstSlider? :type Boolean) (NewFirstValue :type Float%20%28single-precision%29) (NewSecondValue :type Float%20%28single-precision%29))
  (CallFunction|SetRearGunElevation NewFirstValue)
  (CallFunction|SetRearGunBaseRotation NewSecondValue))

(event EventSetTwinSliderVariable3
  (params (bFirstSlider? :type Boolean) (NewFirstValue :type Float%20%28single-precision%29) (NewSecondValue :type Float%20%28single-precision%29))
  (CallFunction|SetFrontLauncherElevation NewFirstValue)
  (CallFunction|SetFrontLauncherBaseRotation NewSecondValue))

(event EventSetTwinSliderVariable4
  (params (bFirstSlider? :type Boolean) (NewFirstValue :type Float%20%28single-precision%29) (NewSecondValue :type Float%20%28single-precision%29))
  (CallFunction|SetRearLauncherElevation NewFirstValue)
  (CallFunction|SetRearLauncherBaseRotation NewSecondValue))

(event EventSetTwinSliderVariable5
  (params (bFirstSlider? :type Boolean) (NewFirstValue :type Float%20%28single-precision%29) (NewSecondValue :type Float%20%28single-precision%29))
  (Utilities|FlowControl|Sequence
    (:then_0
      (CallFunction|SetFrontLeftGunElevation NewFirstValue)
      (CallFunction|SetFrontRightGunElevation NewFirstValue)
      (CallFunction|SetRearLeftGunElevation NewFirstValue)
      (CallFunction|SetRearRightGunElevation NewFirstValue)
      (CallFunction|SetLeftRocketElevation NewFirstValue)
      (CallFunction|SetRightRocketElevation NewFirstValue))
    (:then_1
      (CallFunction|SetFrontLeftGunBaseRotation NewSecondValue)
      (CallFunction|SetFrontRightGunBaseRotation NewSecondValue)
      (CallFunction|SetRearLeftGunBaseRotation NewSecondValue)
      (CallFunction|SetRearRightGunBaseRotation NewSecondValue)
      (CallFunction|SetLeftRocketBaseRotation NewSecondValue)
      (CallFunction|SetRightRocketBaseRotation NewSecondValue))))

(fn ConstructionScript
  (|CallParentFunction))